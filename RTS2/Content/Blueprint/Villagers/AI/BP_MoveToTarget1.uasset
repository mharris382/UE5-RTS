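; BP_MoveToTarget1 is a villager move-target actor that draws navigation paths from pawns to its location using Niagara.
; AssignOwner stores a pawn and starts a looping timer on UpdatePath, which finds a navmesh path, pins its endpoints and feeds the points to Niagara's TargetPath array.
; UpdatePaths does likewise per pawn through MoveLines' child components, but nothing here calls it, and the multi-pawn events are empty.
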(event `Assign Pawns`
  (params (pawns :type "Array of Pawn Object Reference")))

(event `Destroy Lines`)

(event `Create Lines`)

(fn `AssignOwner`
  (params (pawn :type "Pawn Object Reference"))
  (bind _output_get (set `self.owner pawn` pawn))
  (`/Engine/EditorBlueprintResources/StandardMacros.IsValid` _output_get
    (:`Is Valid`
      (bind _returnvalue (`KismetSystemLibrary.K2_SetTimer` null "UpdatePath" 0.2 true))
      (set `self.update path timer` _returnvalue))))

(fn `UpdatePath`
  (locals (path :type "Array of Vector Structure"))
  (bind _returnvalue (`self.K2_GetActorLocation`))
  (bind _owner_pawn (`self.owner pawn`)
    (:`then`
      (bind _returnvalue_2 (`self.K2_GetActorLocation` _owner_pawn))
      (bind _returnvalue_3 (`NavigationSystemV1.FindPathToLocationSynchronously` _returnvalue_2 _returnvalue null null))
      (set `local.path` (`NavigationPath.PathPoints` _returnvalue_3))
      (`KismetArrayLibrary.Array_Set` (`local.path`) 0 _returnvalue_2)
      (`KismetArrayLibrary.Array_Set` (`local.path`) (- (`KismetArrayLibrary.Array_Length` (`local.path`)) 1) _returnvalue)
      (`NiagaraDataInterfaceArrayFunctionLibrary.SetNiagaraArrayVector` (`self.Niagara`) "TargetPath" (`local.path`)))
    (:`else`)))

(fn `UpdatePaths`
  (locals (`cur path` :type "Array of Vector Structure"))
  (bind _returnvalue (`self.K2_GetActorLocation`))
  (bind _cur_path (`local.cur path`))
  (for (_array_element _array_index) (`self.pawns`)
    (bind _returnvalue_2 (`self.K2_GetActorLocation` _array_element))
    (bind _returnvalue_3 (`NavigationSystemV1.FindPathToLocationSynchronously` _returnvalue_2 _returnvalue null null))
    (bind _pathpoints (`NavigationPath.PathPoints` _returnvalue_3))
    (set `local.cur path` _pathpoints)
    (bind (_asniagara_particle_system_component _bsuccess) (cast `NiagaraComponent` (`|GetArrayItem` (`SceneComponent.GetChildrenComponents` (`self.move lines`) false) _array_index) :!pure true))
    (if (and _bsuccess (> (`KismetArrayLibrary.Array_LastIndex` _pathpoints) 0))
      (`KismetArrayLibrary.Array_Set` _cur_path 0 _returnvalue_2)
      (`KismetArrayLibrary.Array_Set` _cur_path (`KismetArrayLibrary.Array_Length` (`local.cur path`)) _returnvalue)
      (`NiagaraDataInterfaceArrayFunctionLibrary.SetNiagaraArrayVector` _asniagara_particle_system_component "TargetPath" (`local.cur path`)))))

(fn `UserConstructionScript`)