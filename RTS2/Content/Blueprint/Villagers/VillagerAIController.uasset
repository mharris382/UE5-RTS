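; AI controller for villagers that keeps the Blackboard in sync with the possessed villager and world state.
; On possess it caches the BP_Villager and binds to its task and home change events.
; Task changes only store the job name and behavior tree, while home changes write to the Blackboard.
; Tick also polls the villager's current building and home, plus the game mode's nighttime flag, into Blackboard keys.
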(event `self.ReceiveTick`
  (params (DeltaSeconds :type "Float (single-precision)"))
  (bind _blackboard (`self.Blackboard`))
  (`|ExecutionSequence`
    (:`then_0`
      (bind _villager (`self.Villager`)
        (:`then`
          (bind (_is_inside _building) (`/Game/Blueprint/BPI_Agent.IsInsideBuilding` _villager))
          (`BlackboardComponent.SetValueAsObject` _blackboard "Inside Building" _building)
          (bind (_has_home _home_building) (`/Game/Blueprint/BPI_Agent.GetHomeAssignment` _villager))
          (`BlackboardComponent.SetValueAsObject` _blackboard "Home" _home_building))
        (:`else`)))
    (:`then_1`
      (bind _asbp_gm (cast `/Game/Blueprint/Core/GameMode/BP_GM` (`GameplayStatics.GetGameMode`)))
      (`BlackboardComponent.SetValueAsBool` (`self.Blackboard`) "Is Night" (`/Game/Blueprint/Core/GameMode/BP_GM.is nighttime` _asbp_gm)))))

(event `self.ReceivePossess`
  (params (PossessedPawn :type "Pawn Object Reference"))
  (bind _asbp_villager (cast `/Game/Blueprint/Villagers/BP_Villager` PossessedPawn))
  (set `self.Villager` _asbp_villager)
  (add `/Game/Blueprint/Villagers/BP_Villager.OnTaskChanged` (`self.Villager`) (delegate `Update Job`))
  (add `/Game/Blueprint/Villagers/BP_Villager.OnHomeChanged` (`self.Villager`) (delegate `Update Home`)))

(event `Update Job`
  (params (`Job Name` :type Name) (`Job Behavior Tree` :type "BehaviorTree Object Reference"))
  (set `self.Job Name` `Job Name`)
  (set `self.Job Behavior Tree` `Job Behavior Tree`))

(event `Update Home`
  (params (`home building` :type "/Game/Blueprint/Interactable/Building/BP_BuildingBase Object Reference"))
  (`BlackboardComponent.SetValueAsObject` (`AIBlueprintHelperLibrary.GetBlackboard` null) (`self.Home Key Name`) `home building`))

(fn `UserConstructionScript`)