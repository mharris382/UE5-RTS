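; BP_Flower_Spawner scatters instanced meshes, flowers by its name, over the ground around the actor.
; Its construction script clears the Hierarchical Instanced Static Mesh, then adds a random number of instances between SpawnMin and SpawnMax.
; Each takes a random horizontal offset within Radius and line-traces downward on Visibility to sit on the hit surface.
; A missed trace falls back to a random point at actor height.
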(fn `UserConstructionScript`
  (bind _returnvalue (+ (* (`KismetMathLibrary.Normal` (* (`KismetMathLibrary.RandomUnitVector`) (1.0 1.0 0.0))) (`KismetMathLibrary.RandomFloatInRange` 0.0 (`self.radius`))) (`self.K2_GetActorLocation`)))
  (`InstancedStaticMeshComponent.ClearInstances` (`self.HierarchicalInstancedStaticMesh`))
  (for _ (range (+ (`KismetMathLibrary.RandomIntegerInRange` (`self.spawn min`) (`self.spawn max`)) 1))
    (bind _outhit (`KismetSystemLibrary.LineTraceSingle` _returnvalue (+ _returnvalue (0.0 0.0 -1000.0)) "TraceTypeQuery1"))
    (bind (_bblockinghit _binitialoverlap _time _distance _location) (`GameplayStatics.BreakHitResult` _outhit))
    (`InstancedStaticMeshComponent.AddInstance` (`self.HierarchicalInstancedStaticMesh`) (`KismetMathLibrary.MakeTransform` (`KismetMathLibrary.SelectVector` _location _returnvalue _bblockinghit) (struct) (1.0 1.0 1.0)) true)))