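; Agent function library that packs a villager actor's state into an STVillager struct.
; GetVillagerData reads behavior and home through BPI_Agent and the occupied building from an optional AgentBuildingOccupancy component, storing buildings as IDs with -1 for none.
; An invalid actor or one without the interface returns Valid false with default data.
; AssignHomeBuilding, TryEnterBuilding and ExitBuilding are empty stubs.
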(fn `AssignHomeBuilding`
  (params (building :type "/Game/Blueprint/Interactable/Building/BP_BuildingBase Object Reference")))

(fn `ExitBuilding`
  (params (building :type "/Game/Blueprint/Interactable/Building/BP_BuildingBase Object Reference")))

(fn `GetVillagerData`
  (params (actor :type "Actor Object Reference"))
  (returns (valid :type Boolean) (`villager data` :type "/Game/Blueprint/Core/Save/ST_Villager Structure"))
  (bind _returnvalue (`Actor.K2_GetActorLocation` actor))
  (bind _returnvalue_2 (`Actor.GetComponentByClass` actor "/Game/Blueprint/Villagers/Components/AgentBuildingOccupancy.AgentBuildingOccupancy_C"))
  (`/Engine/EditorBlueprintResources/StandardMacros.IsValid` actor
    (:`Is Valid`
      (bind _asbpi_agent (cast `/Game/Blueprint/BPI_Agent` actor)
        (:`then`
          (bind _task (`/Game/Blueprint/BPI_Agent.GetCurrentBehavior` _asbpi_agent))
          (bind (_has_home _home_building) (`/Game/Blueprint/BPI_Agent.GetHomeAssignment` _asbpi_agent))
          (`/Engine/EditorBlueprintResources/StandardMacros.IsValid` _returnvalue_2
            (:`Is Valid`
              (bind (_is_inside _building) (`/Game/Blueprint/BPI_Agent.IsInsideBuilding` _returnvalue_2))
              (bind _returnvalue_3 (`KismetMathLibrary.SelectInt` (`/Game/Blueprint/Interactable/BP_Interactable.Get ID` _home_building) -1 (and _has_home (`KismetSystemLibrary.IsValid` _home_building))))
              (return true (make `/Game/Blueprint/Core/Save/ST_Villager` _returnvalue _task (struct) _returnvalue_3 (`KismetMathLibrary.SelectInt` (`/Game/Blueprint/Interactable/BP_Interactable.Get ID` _building) -1 (and _is_inside (`KismetSystemLibrary.IsValid` _building))))))
            (:`Is Not Valid`
              (return true (make `/Game/Blueprint/Core/Save/ST_Villager` _returnvalue _task (struct) _returnvalue_3 -1)))))
        (:`CastFailed`
          _)))
    (:`Is Not Valid`
      _))
  (return false (make `/Game/Blueprint/Core/Save/ST_Villager` (0.0 0.0 0.0))))

(fn `TryEnterBuilding`
  (params (building :type "/Game/Blueprint/Interactable/Building/BP_BuildingBase Object Reference"))
  (returns (success :type Boolean))
  (return false))