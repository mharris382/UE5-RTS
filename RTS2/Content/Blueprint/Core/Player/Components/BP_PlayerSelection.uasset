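; BP_PlayerSelection is a player selection component that turns pawn drags and focus changes into game actions.
; Dragging a BP_Wizard to a location issues it a move command, while dragging one onto an actor only prints an on-screen "use" message so far.
; Focus changes set or clear the focus target on BP_GM, fetched by casting the game mode.
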(event `self.ReceiveTick`
  (params (DeltaSeconds :type "Float (single-precision)"))
  (`parent.ReceiveTick` DeltaSeconds))

(event `self.OnPawnDraggedToActor`
  (params (draggedPawn :type "Pawn Object Reference") (draggedOntoActor :type "Actor Object Reference"))
  (cast `/Game/Blueprint/Wizards/BP_Wizard` draggedPawn)
  (`KismetSystemLibrary.PrintText` (`|FormatText` "Tell wizard to use {0}" (`KismetSystemLibrary.GetDisplayName` draggedOntoActor)) true true (struct :`G` 1.0 :`B` 0.132557 :`A` 1.0) 5.0))

(event `self.OnPawnDraggedToLocation`
  (params (draggedPawn :type "Pawn Object Reference") (dragEndPosition :type "Vector Structure"))
  (bind _asbp_wizard (cast `/Game/Blueprint/Wizards/BP_Wizard` draggedPawn))
  (`/Game/Blueprint/Wizards/BP_Wizard.GiveMoveToLocationCommand` _asbp_wizard dragEndPosition))

(event `self.FocusedActorChanged`
  (params (actor :type "Actor Object Reference"))
  (`/Engine/EditorBlueprintResources/StandardMacros.IsValid` actor
    (:`Is Valid`
      (bind _asbp_gm (`self.Get GM`))
      (`/Game/Blueprint/Core/GameMode/BP_GM.Set Focus Target` _asbp_gm actor))
    (:`Is Not Valid`
      (bind _asbp_gm_2 (`self.Get GM`))
      (`/Game/Blueprint/Core/GameMode/BP_GM.Clear Focus Target` _asbp_gm_2))))