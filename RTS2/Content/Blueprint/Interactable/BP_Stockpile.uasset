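; BP_Stockpile is an interactable actor that stores resource amounts by type in a map, optionally restricted to allowed types.
; LoadResources sets contents and filter, with an empty filter accepting everything.
; Add and remove functions report success and a remainder, with no capacity limit; short removals delete the entry before computing the remainder from it.
; Loading and successful or partial changes call ResourcesChanged, an empty event here.
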(event `/Game/Blueprint/Interactable/BPI_Stockpile.LoadResources`
  (params (resources :type "Map of /Game/Blueprint/Interactable/Extras/E_ResourceType Enum to Integer" :default _) (`allowed types` :type "Array of /Game/Blueprint/Interactable/Extras/E_ResourceType Enum (by ref)" :default _))
  (set `self.stored resources` resources)
  (bind _output_get (set `self.allowed resources` `allowed types`))
  (set `self.allows all resources` (== (`KismetArrayLibrary.Array_Length` _output_get) 0))
  (`self.Resources Changed`))

(event `Resources Changed`)

(fn `CanAddResource`
  (params (`resource type` :type "/Game/Blueprint/Interactable/Extras/E_ResourceType Enum" :default "NewEnumerator5") (amount :type Integer))
  (returns (`can add` :type Boolean))
  (return (or (`self.allows all resources`) (`KismetArrayLibrary.Array_Contains` (`self.allowed resources`) `resource type`))))

(fn `CanRemoveResource`
  (params (`resource type` :type "/Game/Blueprint/Interactable/Extras/E_ResourceType Enum" :default "NewEnumerator5") (`amount to remove` :type Integer))
  (returns (`can remove` :type Boolean))
  (bind (_value _returnvalue) (`BlueprintMapLibrary.Map_Find` (`self.stored resources`) `resource type`))
  (if _returnvalue
    (return (>= _value `amount to remove`))
    (else
      (return false))))

(fn `GetResources`
  (returns (stored :type "Map of /Game/Blueprint/Interactable/Extras/E_ResourceType Enum to Integer") (`allowed types` :type "Array of /Game/Blueprint/Interactable/Extras/E_ResourceType Enum"))
  (return (`self.stored resources`) (select `bool` (or (`self.allows all resources`) (== (`KismetArrayLibrary.Array_Length` (`self.allowed resources`)) 0)) :`false` (`self.allowed resources`) :`true` (`|MakeArray`))))

(fn `TryAddResource`
  (params (`resource type` :type "/Game/Blueprint/Interactable/Extras/E_ResourceType Enum" :default "NewEnumerator5") (`amount to add` :type Integer))
  (returns (`added fully` :type Boolean) (remainder :type Integer))
  (bind (_value _returnvalue) (`BlueprintMapLibrary.Map_Find` (`self.stored resources`) `resource type`))
  (bind _can_add (`self.CanAddResource` `resource type` `amount to add`))
  (if _can_add
    (`BlueprintMapLibrary.Map_Add` (`self.stored resources`) `resource type` (`KismetMathLibrary.SelectInt` (+ _value `amount to add`) `amount to add` _returnvalue))
    (`self.Resources Changed`)
    (return true 0)
    (else
      (return false `amount to add`))))

(fn `TryRemoveResource`
  (params (`resource type` :type "/Game/Blueprint/Interactable/Extras/E_ResourceType Enum" :default "NewEnumerator5") (`amount to remove` :type Integer))
  (returns (`removed fully` :type Boolean) (remainder :type Integer))
  (bind _stored_resources (`self.stored resources`))
  (bind (_value _returnvalue) (`BlueprintMapLibrary.Map_Find` (`self.stored resources`) `resource type`))
  (if _returnvalue
    (if (>= _value `amount to remove`)
      (`BlueprintMapLibrary.Map_Add` _stored_resources `resource type` (- _value `amount to remove`))
      (`self.Resources Changed`)
      (return true 0)
      (else
        (`BlueprintMapLibrary.Map_Remove` _stored_resources `resource type`)
        (`self.Resources Changed`)
        (return false (- `amount to remove` _value))))
    (else
      (return false `amount to remove`))))

(fn `UserConstructionScript`
  (`parent.UserConstructionScript`))