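; Save-fix actor that guarantees a wizard exists after a game load.
; On BeginPlay, if BP_GM is loading, it binds a check to the game mode's OnLoadCompleted event.
; When the load completes, the check asks BP_GM to spawn a wizard if no Wizard actors are in the world.
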(event `self.ReceiveBeginPlay`
  (bind _asbp_gm (cast `/Game/Blueprint/Core/GameMode/BP_GM` (`GameplayStatics.GetGameMode`)))
  (if (`/Game/Blueprint/Core/GameMode/BP_GM.loading` _asbp_gm)
    (add `/Game/Blueprint/Core/GameMode/BP_GM.On Load Completed` _asbp_gm (delegate `Verify First Wizard Exists`))))

(event `Verify First Wizard Exists`
  (bind _outactors (`GameplayStatics.GetAllActorsOfClass` "/Script/RTS2.Wizard"))
  (if (== (`KismetArrayLibrary.Array_Length` _outactors) 0)
    (bind _asbp_gm (cast `/Game/Blueprint/Core/GameMode/BP_GM` (`GameplayStatics.GetGameMode`)))
    (`/Game/Blueprint/Core/GameMode/BP_GM.Spawn Wizard` _asbp_gm)))

(fn `UserConstructionScript`)