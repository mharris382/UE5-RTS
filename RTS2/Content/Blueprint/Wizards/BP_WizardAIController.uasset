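; AI controller for BP_Wizard that runs BT_WizardDefault and feeds its blackboard.
; BeginPlay caches game mode and wizard, then sets the TownHall key, retrying on a looping timer until the town hall exists.
; Tick copies the move target to MoveToLocation, and writes self, current building and home building all to "Inside Building", so the last overwrites the others.
; It also supplies the wizard focus widget.
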(event `self.ReceiveBeginPlay`
  (`self.RunBehaviorTree` "/Game/Blueprint/Wizards/AI/BehaviorTrees/BT_WizardDefault.BT_WizardDefault")
  (bind _asbp_gm (cast `/Game/Blueprint/Core/GameMode/BP_GM` (`GameplayStatics.GetGameMode`)))
  (set `self.BP GameMode` _asbp_gm)
  (bind _asbp_wizard (cast `/Game/Blueprint/Wizards/BP_Wizard` (`self.K2_GetPawn`)))
  (set `self.BP Wizard` _asbp_wizard)
  (`self.Update Town Hall`))

(event `self.ReceiveTick`
  (params (DeltaSeconds :type "Float (single-precision)"))
  (`/Engine/EditorBlueprintResources/StandardMacros.IsValid` (`AIBlueprintHelperLibrary.GetBlackboard` null)
    (:`Is Valid`
      (`self.GetWizard`
        (:`Is Valid`
          (`|ExecutionSequence`
            (:`then_0`
              ;[1 1 1 0.5] Assign self
              (`BlackboardComponent.SetValueAsObject` (`AIBlueprintHelperLibrary.GetBlackboard` null) "Inside Building" (`self.BP Wizard`)))
            (:`then_1`
              ;[1 1 1 0.5] Assign Current Building
              (`BlackboardComponent.SetValueAsObject` (`AIBlueprintHelperLibrary.GetBlackboard` null) "Inside Building" (`/Game/Blueprint/Villagers/Components/AgentBuildingOccupancy.current building` (`/Game/Blueprint/Wizards/BP_Wizard.AgentBuildingOccupancy` (`self.BP Wizard`)))))
            (:`then_2`
              ;[1 1 1 0.5] Assign Home Building
              (`BlackboardComponent.SetValueAsObject` (`AIBlueprintHelperLibrary.GetBlackboard` null) "Inside Building" (`/Game/Blueprint/Wizards/BP_Wizard.Home Building` (`self.BP Wizard`))))
            (:`then_3`
              ;[1 1 1 0.5] Assign Move to Command
              (`BlackboardComponent.SetValueAsObject` (`AIBlueprintHelperLibrary.GetBlackboard` null) "MoveToLocation" (`/Game/Blueprint/Wizards/BP_Wizard.current move target` (`self.BP Wizard`))))))
        (:`CastFailed`
          (`KismetSystemLibrary.PrintText` "AI has no wizard" true true (struct :`R` 1.0 :`B` 0.045438 :`A` 1.0)))))
    (:`Is Not Valid`
      (`KismetSystemLibrary.PrintText` "AI has no blackboard" true true (struct :`R` 1.0 :`B` 0.097106 :`A` 1.0)))))

(event `Update Home`)

(event `Update Town Hall`
  ;[1 1 1 0.5] Set Town Hall Reference on Blackboard
  (bind _success (`self.Try Set TownHall BB Ref`))
  (if (not _success)
    (bind _returnvalue (`KismetSystemLibrary.K2_SetTimerDelegate` (delegate `check for town hall spawned`) 0.1 true))
    (set `self.wait for town hall spawned` _returnvalue)))

(event `check for town hall spawned`
  ;[1 1 1 0.5] Set Town Hall Reference on Blackboard
  (bind _success (`self.Try Set TownHall BB Ref`))
  (if _success
    (`KismetSystemLibrary.K2_ClearAndInvalidateTimerHandle` (`self.wait for town hall spawned`))))

(fn `Get Full Focus Widget`
  (returns (`focus widget` :type "/Game/UI/UI_Elements/FocusTargets/WB_FocusWindow Class Reference"))
  (return "/Game/UI/UI_Elements/FocusTargets/WizardFocus/WB_WizardFocus.WB_WizardFocus_C"))

(fn `Try Set TownHall BB Ref`
  (returns (success :type Boolean))
  (bind _returnvalue (`AIBlueprintHelperLibrary.GetBlackboard` null))
  (bind _bp_gamemode (`self.BP GameMode`))
  (bind _town_hall (`/Game/Blueprint/Core/GameMode/BP_GM.Town Hall` _bp_gamemode))
  (`/Engine/EditorBlueprintResources/StandardMacros.IsValid` _returnvalue
    (:`Is Valid`
      (`/Engine/EditorBlueprintResources/StandardMacros.IsValid` _bp_gamemode
        (:`Is Valid`
          (`/Engine/EditorBlueprintResources/StandardMacros.IsValid` _town_hall
            (:`Is Valid`
              (`BlackboardComponent.SetValueAsObject` _returnvalue "TownHall" _town_hall)
              (return true))
            (:`Is Not Valid`
              _)))
        (:`Is Not Valid`
          _)))
    (:`Is Not Valid`
      _))
  (return false))

(fn `UserConstructionScript`)