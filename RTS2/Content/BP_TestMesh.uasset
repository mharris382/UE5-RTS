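; Procedurally builds a seeded, island-like landmass with Geometry Script, optionally at construction via PreConstruct.
; CreateMesh scatters random cones and cylinders, applies Perlin noise, then solidifies, smooths, tessellates, plane-cuts top and bottom, and planar-projects UVs.
; Solidify resolution and tessellation drop on Android, Switch and iOS through PlatformSwitch.
; Afterwards it releases compute meshes, nudges the actor upward and randomizes the MPC_Landscape GrassColour hue from the same seed.
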(fn `Create Mesh`
  (bind _points (`self.points`))
  (bind _dyn_mesh (`self.dyn mesh`))
  (bind _radius (`self.radius`))
  (bind (_spawn_size_x _spawn_size_y) (`KismetMathLibrary.BreakVector2D` (`self.spawn size`)))
  (bind (_returnvalue_x _returnvalue_y) (`KismetMathLibrary.BreakVector` (* (`KismetMathLibrary.RandomUnitVectorFromStream` (`self.seed`)) (/ (`self.spawn dist`) 2.0))))
  (bind _returnvalue (`BaseDynamicMeshComponent.GetDynamicMesh` (`self.DynamicMeshComponent`)))
  (bind _output_get (set `self.dyn mesh` _returnvalue))
  (`DynamicMesh.Reset` _output_get)
  (`KismetArrayLibrary.Array_Clear` (`self.points`))
  (`|ExecutionSequence`
    (:`then_0`
      (for _ (range (+ (`self.count`) 1))
        (set `self.radius` (`KismetMathLibrary.RandomFloatInRangeFromStream` (`self.seed`) _spawn_size_x _spawn_size_y))
        (bind _returnvalue_2 (`KismetArrayLibrary.Array_Add` _points (`KismetMathLibrary.MakeVector` _returnvalue_x _returnvalue_y)))
        (if (> (`KismetMathLibrary.RandomFloatInRangeFromStream` (`self.seed`) 0.0 1.0) (`self.cylinder chance`))
          (bind (_output_x _output_y) (`KismetMathLibrary.BreakVector` (`|GetArrayItem` _points _returnvalue_2)))
          (bind _returnvalue_3 (`KismetMathLibrary.MakeTransform` (`KismetMathLibrary.MakeVector` _output_x _output_y -800.0)))
          (`GeometryScriptLibrary_MeshPrimitiveFunctions.AppendCone` _dyn_mesh (struct) _returnvalue_3 _radius (/ _radius (`self.cone steepness`)) 1300.0 32 1 true "Base" null)
          (else
            (`GeometryScriptLibrary_MeshPrimitiveFunctions.AppendCylinder` _dyn_mesh (struct) _returnvalue_3 (`self.radius`) 1300.0 32 1 true "Base" null)))
        (`GeometryScriptLibrary_MeshDeformFunctions.ApplyPerlinNoiseToMesh` _dyn_mesh (struct) (struct) null))
      (bind _returnvalue_4 (`GeometryScriptLibrary_MeshVoxelFunctions.ApplyMeshSolidify` (`self.dyn mesh`) (make `GeometryScriptSolidifyOptions` (make `GeometryScript3DGridParameters` "GridResolution" (`self.Grid Cell Size`) (`self.Platform Switch` 60 50)) 0.5 true 1.0 64) null))
      (bind _returnvalue_5 (`GeometryScriptLibrary_MeshNormalsFunctions.SetPerVertexNormals` _returnvalue_4 null))
      (bind _returnvalue_6 (`GeometryScriptLibrary_MeshDeformFunctions.ApplyIterativeSmoothingToMesh` _returnvalue_5 (struct) (make `GeometryScriptIterativeMeshSmoothingOptions` (`self.Smoothing Num Iterations`)) null))
      (bind _returnvalue_7 (`GeometryScriptLibrary_MeshSubdivideFunctions.ApplyPNTessellation` _returnvalue_6 (struct) (`self.Platform Switch` 0 2) null))
      (bind _returnvalue_8 (`GeometryScriptLibrary_MeshBooleanFunctions.ApplyMeshPlaneCut` _returnvalue_7 (`KismetMathLibrary.MakeTransform` (0.0 0.0 -390.0) (struct :`Roll` 180.0)) (make `GeometryScriptMeshPlaneCutOptions` false false) null))
      (bind _returnvalue_9 (`GeometryScriptLibrary_MeshBooleanFunctions.ApplyMeshPlaneCut` _returnvalue_8 (`KismetMathLibrary.MakeTransform` (0.0 0.0 0.0)) (struct) null))
      (`GeometryScriptLibrary_MeshUVFunctions.SetMeshUVsFromPlanarProjection` _returnvalue_9 0 (`KismetMathLibrary.MakeTransform` (0.0 0.0 0.0) (struct) (100.0 100.0 100.0)) (struct) null))
    (:`then_1`
      (`self.ReleaseAllComputeMeshes`)
      (`self.K2_AddActorWorldOffset` (0.0 0.0 0.05)))
    (:`then_2`
      (bind _returnvalue_10 (`KismetMaterialLibrary.GetVectorParameterValue` "/Game/Misc/MPC_Landscape.MPC_Landscape" "GrassColour"))
      (bind (_h _s _v _a) (`KismetMathLibrary.RGBToHSV` _returnvalue_10))
      (`KismetMaterialLibrary.SetVectorParameterValue` "/Game/Misc/MPC_Landscape.MPC_Landscape" "GrassColour" (`KismetMathLibrary.HSVToRGB` (+ 102.999725 (`KismetMathLibrary.RandomFloatInRangeFromStream` (`self.seed`) 0.0 90.0)) _s _v _a)))))

(fn `Platform Switch`
  (params (low :type Integer) (high_end :type Integer))
  (returns (NewParam :type Integer))
  (bind _returnvalue (`GameplayStatics.GetPlatformName`))
  (return (`KismetMathLibrary.SelectInt` low high_end (or (`KismetStringLibrary.EqualEqual_StrStr` _returnvalue "Android") (`KismetStringLibrary.EqualEqual_StrStr` _returnvalue "Switch") (`KismetStringLibrary.EqualEqual_StrStr` _returnvalue "IOS")))))

(fn `UserConstructionScript`
  (if (`self.pre construct`)
    (`self.Create Mesh`)))