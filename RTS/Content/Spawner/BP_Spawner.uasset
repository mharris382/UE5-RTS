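; Spawner that scatters actors and instanced static meshes in biome clusters across the navmesh, with seeded per-cluster counts.
; Soft classes async load one by one at BeginPlay, gating spawning on low-end platforms.
; A looping timer spawns one type per pass once loading and nav builds finish, letting the navmesh rebuild between types to reduce overlap.
; Actor types precede mesh instances unless mesh-only, then optional completion messages notify GameInstance and GameMode.
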(event `AsyncLoad Classes`
  ;[1 1 1] Get each soft class reference and async load them ready for spawning. The boolean is used as a blocker to stop spawning until all classes are loaded. This is needed for lower end platforms like mobile.
  (set `self.Class Ref Index` 0)
  (set `self.Async Complete` false)
  (`|LoadAssetClass` (`.ClassRef_13_89B0B33C423AF7627034AF87E3308B2B` (break `/Game/Spawner/ST_SpawnData` (`|GetArrayItem` (`self.SpawnTypes`) (`self.Class Ref Index`)))) :!label _label
    (:`Completed`
      (bind _result (`/Engine/EditorBlueprintResources/StandardMacros.IncrementInt` (`self.Class Ref Index`))
        (:`  `
          (if (> _result (`KismetArrayLibrary.Array_LastIndex` (`self.SpawnTypes`)))
            (set `self.Async Complete` true)
            (else
              (`self.Async Class`))))))))

(event `Async Class`
  ;[1 1 1] Get each soft class reference and async load them ready for spawning. The boolean is used as a blocker to stop spawning until all classes are loaded. This is needed for lower end platforms like mobile.
  (goto _label))

(event `Spawn Mesh Only`
  ;[1 1 1] Control when actors are spawned into game
  (set `self.Actor Switch` false)
  ;[1 1 1] Retrigerrable Timer that waits for nav system to be built and soft classes to be loaded. This is needed because the assets we spawn will cause the nav mesh to be rebuilt. Rebuilding the nav mesh will help reduce overlapping assets
  (`KismetSystemLibrary.DelayUntilNextTick` :!label _label_2)
  (set `self.Counter` 0)
  (set `self.Index Counter` 0)
  (bind _returnvalue (`KismetSystemLibrary.K2_SetTimerDelegate` (delegate `Ready To Spawn`) 0.5 true -0.5))
  (set `self.Nav Check Handle` _returnvalue))

(event `self.ReceiveBeginPlay`
  ;[1 1 1] Load Soft Class Refs
  (`self.AsyncLoad Classes`)
  ;[1 1 1] Control when actors are spawned into game
  (if (`self.Auto Spawn`)
    (goto _label_2)))

(event `Spawn Random`
  ;[1 1 1] Control when actors are spawned into game
  (goto _label_2))

(event `Ready To Spawn`
  (bind _index_counter (`self.Index Counter`))
  (bind _index_counter_2 (`self.Index Counter`))
  (bind _output (`|GetArrayItem` (`self.SpawnTypes`) (`self.Index Counter`)))
  (bind (_output_classref _output_biomescale _output_biomecount _output_spawnperbiome) (break `/Game/Spawner/ST_SpawnInstance` (`|GetArrayItem` (`self.SpawnInstances`) (`self.Index Counter`))))
  ;[1 1 1] Retrigerrable Timer that waits for nav system to be built and soft classes to be loaded. This is needed because the assets we spawn will cause the nav mesh to be rebuilt. Rebuilding the nav mesh will help reduce overlapping assets
  (if (and (not (`NavigationSystemV1.IsNavigationBeingBuilt` (`NavigationSystemV1.GetNavigationSystem`))) (`self.Async Complete`))
    (`KismetSystemLibrary.K2_PauseTimerHandle` (`self.Nav Check Handle`))
    ;[1 1 1] Once finished spawning BP's, spawn the instanced static mesh array
    (if (`self.Actor Switch`)
      ;[1 1 1] Spawn of Class
      (`self.SpawnAssets` (`|ConvertAsset` (`.ClassRef_13_89B0B33C423AF7627034AF87E3308B2B` (break `/Game/Spawner/ST_SpawnData` _output))) _output)
      ;[1 1 1] Switch Class After Pause
      (`/Engine/EditorBlueprintResources/StandardMacros.IncrementInt` _index_counter_2
        (:`  `
          (if (>= _index_counter_2 (`KismetArrayLibrary.Array_Length` (`self.SpawnTypes`)))
            (set `self.Index Counter` 0)
            (set `self.Actor Switch` false))
          (`KismetSystemLibrary.K2_UnPauseTimerHandle` (`self.Nav Check Handle`))))
      (else
        ;[1 1 1] Spawn Instances
        (bind _returnvalue (`AddComponent|NODE_AddInstancedStaticMeshComponent-0`))
        (`StaticMeshComponent.SetStaticMesh` _returnvalue _output_classref)
        (`self.SpawnInst` _returnvalue _output_biomescale _output_biomecount _output_spawnperbiome)
        (`/Engine/EditorBlueprintResources/StandardMacros.IncrementInt` _index_counter
          (:`  `
            (if (>= _index_counter (`KismetArrayLibrary.Array_Length` (`self.SpawnInstances`)))
              (if (`self.Call Save`)
                (`self.Finished Spawning`))
              (else
                (`KismetSystemLibrary.K2_UnPauseTimerHandle` (`self.Nav Check Handle`))))))))))

(event `Finished Spawning`
  ;[1 1 1] Send Finished Spawning Event
  (message `/Game/Blueprint/Core/Save/BPI_GI.Update All Interactables` (`GameplayStatics.GetGameInstance`))
  (message `/Game/Misc/BPI_IslandPlugin.Spawning Complete` (`GameplayStatics.GetGameMode`)))

(fn `Load Spawn`
  (params (NewParam :type "/Game/Blueprint/Core/Save/ST_SaveInteract Structure")))

(fn `SpawnAssets`
  (params (Class :type "Actor Object Reference") (`Spawn Params` :type "/Game/Spawner/ST_SpawnData Structure"))
  (locals (Pos :type "Vector Structure" :default (0.0 0.0 0.0)) (SpawnPos :type "Vector Structure" :default (0.0 0.0 0.0)) (Counter :type Integer))
  (bind ((`RandomRotationRange_19_D40763014C0AEE20FB81F0BF26C6AC3D` _randomrotationrange) (`ScaleRange_18_439428C84034733625BCEF875A49A74E` _scalerange)) (break `/Game/Spawner/ST_SpawnData` (`local.Spawn Params`)))
  ;[1 1 1] Loop Of Initial Biome Points
  (for _ (range (+ (`.BiomeCount_9_2C7D811540AF169A83AD5AAAB0B4412E` (break `/Game/Spawner/ST_SpawnData` `Spawn Params`)) 1))
    (bind _randomlocation (`NavigationSystemV1.K2_GetRandomLocationInNavigableRadius` (`KismetMathLibrary.MakeVector` 0.0) 10000.0 (`self.Nav Data`) null))
    (set `local.Pos` _randomlocation)
    ;[1 1 1] Pick Points around Biome Points
    (for _ (range (+ (`KismetMathLibrary.RandomIntegerInRangeFromStream` (`self.Seed`) 0 (`.SpawnPerBiome_10_1900F06D464B41C659F65D91568D0A73` (break `/Game/Spawner/ST_SpawnData` (`local.Spawn Params`)))) 1))
      (bind _randomlocation_2 (`NavigationSystemV1.K2_GetRandomLocationInNavigableRadius` (`local.Pos`) (`.BiomeScale_12_EDD71B5E4CBA6714CA44EA865630E4C3` (break `/Game/Spawner/ST_SpawnData` (`local.Spawn Params`))) (`self.Nav Data`) null))
      (bind _output_get (set `local.SpawnPos` _randomlocation_2))
      ;[1 1 1] Spawn Actor
      (bind _returnvalue (`|SpawnActorFromClass` (`local.Class`) (`KismetMathLibrary.MakeTransform` (`/Game/Blueprint/Core/GameMode/BPF_Cropout.Stepped Position` _output_get) (`KismetMathLibrary.MakeRotator` 0.0 0.0 (`KismetMathLibrary.RandomFloatInRange` 0.0 _randomrotationrange)) (`KismetMathLibrary.Conv_DoubleToVector` (`KismetMathLibrary.RandomFloatInRange` 1.0 (+ _scalerange 1.0)))) "AlwaysSpawn" "SelectDefaultAtRuntime" null null))
      (bind _result (`/Engine/EditorBlueprintResources/StandardMacros.IncrementInt` (`local.Counter`))))))

(fn `SpawnInst`
  (params (Class :type "InstancedStaticMeshComponent Object Reference") (Radius :type "Float (single-precision)") (`Biome Count` :type Integer) (`Max Spawn` :type Integer))
  (locals (Pos :type "Vector Structure" :default (0.0 0.0 0.0)) (SpawnPos :type "Vector Structure" :default (0.0 0.0 0.0)) (Counter :type Integer))
  (bind (_spawnpos_x _spawnpos_y) (`KismetMathLibrary.BreakVector` (`local.SpawnPos`)))
  ;[1 1 1] Loop Of Initial Biome Points
  (for _ (range (+ `Biome Count` 1))
    (bind _randomlocation (`NavigationSystemV1.K2_GetRandomLocationInNavigableRadius` (`KismetMathLibrary.MakeVector` 0.0) 10000.0 (`self.Nav Data`) null))
    (set `local.Pos` _randomlocation)
    ;[1 1 1] Pick Points around Biome Points
    (for _ (range (+ (`KismetMathLibrary.RandomIntegerInRangeFromStream` (`self.Seed`) 0 (`local.Max Spawn`)) 1))
      (bind _randomlocation_2 (`NavigationSystemV1.K2_GetRandomLocationInNavigableRadius` (`local.Pos`) (`local.Radius`) (`self.Nav Data`) null))
      (set `local.SpawnPos` _randomlocation_2)
      (`InstancedStaticMeshComponent.AddInstance` (`local.Class`) (`KismetMathLibrary.MakeTransform` (`KismetMathLibrary.MakeVector` _spawnpos_x _spawnpos_y) (`KismetMathLibrary.MakeRotator` 0.0) (`KismetMathLibrary.Conv_DoubleToVector` (`KismetMathLibrary.Lerp` 0.8 1.5 (/ (`KismetMathLibrary.VSize` (- (`local.Pos`) (`local.SpawnPos`))) (`local.Radius`))))) true)
      (`/Engine/EditorBlueprintResources/StandardMacros.IncrementInt` (`local.Counter`)))))

(fn `UserConstructionScript`)