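; BP_SaveGM generates a villager name that aims not to duplicate any name in the Villagers list.
; GenerateNewVilliageName takes a first and a last name from two randomly picked data table rows and compares the pair against existing villagers.
; On a clash it steps both row indices with wraparound and retests; a failed row lookup returns "John Doe".
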(fn `Generate New Villiage Name`
  (returns (`new name` :type "/Game/Blueprint/Villagers/S_Name Structure"))
  (locals (dt :type "DataTable Object Reference" :default "/Script/Engine.DataTable'/Game/Blueprint/Villagers/DT_RandomNames.DT_RandomNames'") (`total count` :type Integer :default 990) (`name exists` :type Boolean) (`first name row` :type Integer :default 0) (`second name row` :type Integer :default 0) (`output name` :type "/Game/Blueprint/Villagers/S_Name Structure") (`max rows` :type Integer) (tries :type Integer) (rows :type "Array of Name"))
  (bind (_output_name_first _output_name_last) (break `/Game/Blueprint/Villagers/S_Name` (`local.output name`)))
  (bind (_output_name_first_2 _output_name_last_2) (break `/Game/Blueprint/Villagers/S_Name` (`local.output name`)))
  (set `local.name exists` false)
  (bind _outrownames (`DataTableFunctionLibrary.GetDataTableRowNames` (`local.dt`)))
  (set `local.rows` _outrownames)
  (bind _returnvalue (- (`KismetArrayLibrary.Array_Length` _outrownames) 1))
  (set `local.max rows` _returnvalue)
  (set `local.first name row` (`KismetMathLibrary.RandomIntegerInRange` 0 _returnvalue))
  (set `local.second name row` (`KismetMathLibrary.RandomIntegerInRange` 0 _returnvalue))
  (bind _returnvalue_2 (`|GetDataTableRow` (`local.dt`) (`|GetArrayItem` (`local.rows`) (`local.second name row`)))
    (:`then`
      (bind _returnvalue_3 (`|GetDataTableRow` (`local.dt`) (`|GetArrayItem` (`local.rows`) (`local.first name row`)))
        (:`then`
          (set `local.output name` (make `/Game/Blueprint/Villagers/S_Name` (`.First_5_7413D3A04731F9C6F4CE578DEAAC561C` (break `/Game/Blueprint/Villagers/S_Name` _returnvalue_3)) (`.Last_6_AFFB0AEE4699FD2745B5069FCA690619` (break `/Game/Blueprint/Villagers/S_Name` _returnvalue_2))))
          (set `local.name exists` false)
          (for _array_element (`self.Villagers`)
            (bind (_location _task _name) (break `/Game/Blueprint/Core/Save/ST_Villager` _array_element))
            (if (and (== (break `/Game/Blueprint/Villagers/S_Name` _name) _output_name_first) (== (`.Last_6_AFFB0AEE4699FD2745B5069FCA690619` (break `/Game/Blueprint/Villagers/S_Name` _name)) _output_name_last))
              (set `local.name exists` true)
              (break)))
          (if (`local.name exists`)
            (while (or (`local.name exists`) (< (`local.tries`) 25))
              (set `local.tries` (+ (`local.tries`) 1))
              (set `local.first name row` (mod (+ (`local.first name row`) 1) (`local.max rows`)))
              (set `local.second name row` (mod (+ (`local.second name row`) 1) (`local.max rows`)))
              (bind _returnvalue_4 (`|GetDataTableRow` (`local.dt`) (`|GetArrayItem` (`local.rows`) (`local.second name row`)))
                (:`then`
                  (bind _returnvalue_5 (`|GetDataTableRow` (`local.dt`) (`|GetArrayItem` (`local.rows`) (`local.first name row`)))
                    (:`then`
                      (set `local.output name` (make `/Game/Blueprint/Villagers/S_Name` (`.First_5_7413D3A04731F9C6F4CE578DEAAC561C` (break `/Game/Blueprint/Villagers/S_Name` _returnvalue_5)) (`.Last_6_AFFB0AEE4699FD2745B5069FCA690619` (break `/Game/Blueprint/Villagers/S_Name` _returnvalue_4))))
                      (set `local.name exists` false)
                      (for _array_element_2 (`self.Villagers`)
                        (bind (_location_2 _task_2 _name_2) (break `/Game/Blueprint/Core/Save/ST_Villager` _array_element_2))
                        (if (and (== (break `/Game/Blueprint/Villagers/S_Name` _name_2) _output_name_first_2) (== (`.Last_6_AFFB0AEE4699FD2745B5069FCA690619` (break `/Game/Blueprint/Villagers/S_Name` _name_2)) _output_name_last_2))
                          (set `local.name exists` true)
                          (break)))
                      (if (not (`local.name exists`))
                        (return (`local.output name`))))
                    (:`RowNotFound`
                      (return (make `/Game/Blueprint/Villagers/S_Name` "John" "Doe")))))
                (:`RowNotFound`
                  (return (make `/Game/Blueprint/Villagers/S_Name` "John" "Doe")))))
            (else
              (return (`local.output name`)))))
        (:`RowNotFound`
          (return (make `/Game/Blueprint/Villagers/S_Name` "John" "Doe")))))
    (:`RowNotFound`
      (return (make `/Game/Blueprint/Villagers/S_Name` "John" "Doe")))))