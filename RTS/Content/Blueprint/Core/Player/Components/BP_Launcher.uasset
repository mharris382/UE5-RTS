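; Player launcher component that charges and spawns a BP_Projectile, with launch force scaled by charge time.
; LaunchStart resets the charge, LaunchUpdate accumulates it, and FinishLaunch fires automatically at full charge or when called.
; Spawning uses either a custom transform or a downward-pitched one at the cursor, falling back to the owner, with random horizontal and upward offsets.
; The charge interpolates the projectile's InitialSpeed between minimum and maximum force after spawning.
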(event `Launch Start`
  (if (not (`self.is launching`))
    (set `self.is launching` true)
    (set `self.t` 0.0)))

(event `Launch Update`
  (params (`elapsed time` :type "Float (double-precision)"))
  (if (`self.is launching`)
    (bind _output_get (set `self.t` (+ (/ `elapsed time` (`self.launch max duration`)) (`self.t`))))
    (if (>= _output_get 1.0)
      (`self.Finish Launch`))))

(event `Finish Launch`
  (bind _cursor (`self.cursor`))
  (if (`self.is launching`)
    (set `self.is launching` false)
    (bind _returnvalue (`|SpawnActorFromClass` "/Game/VFX/Test/BP_Projectile.BP_Projectile_C" (`KismetMathLibrary.SelectTransform` (`self.custom transform`) (`KismetMathLibrary.MakeTransform` (+ (`KismetMathLibrary.SelectVector` (`SceneComponent.K2_GetComponentLocation` _cursor) (`Actor.K2_GetActorLocation` (`self.GetOwner`)) (`KismetSystemLibrary.IsValid` _cursor)) (* (* (`KismetMathLibrary.RandomUnitVector`) (1.0 1.0 0.0)) (`self.random offset`)) (* (`KismetMathLibrary.Vector_Up`) (`self.up offset`))) (`KismetMathLibrary.MakeRotator` 0.0 -90.0)) (`self.use custom transform`)) "Undefined" "MultiplyWithRoot" null null))
    (set `ProjectileMovementComponent.InitialSpeed` (`KismetMathLibrary.Lerp` (`self.min launch force`) (`self.max launch force`) (`KismetMathLibrary.FClamp` (`self.t`))) (`/Game/VFX/Test/BP_Projectile.ProjectileMovement` _returnvalue))))