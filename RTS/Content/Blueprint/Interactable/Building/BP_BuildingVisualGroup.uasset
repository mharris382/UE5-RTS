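; Scene component for buildings that shows or hides itself and its children as construction progresses.
; On BeginPlay it binds to the owning BP_BuildingBase's construction update event, doing nothing if the owner is another type.
; Each update applies its Mode: visible only when complete, below a percent threshold, or at and above that threshold.
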(event `self.ReceiveBeginPlay`
  (bind _asbp_building_base (cast `/Game/Blueprint/Interactable/Building/BP_BuildingBase` (`self.GetOwner`)))
  (add `/Game/Blueprint/Interactable/Building/BP_BuildingBase.ConstructionUpdated` _asbp_building_base (delegate `Construction Updated`)))

(event `Construction Updated`
  (params (`Is Construction Completed` :type Boolean) (`Construction Percent` :type "Float (double-precision)"))
  (bind _construction_threshold (`self.Construction Threshold`))
  (switch `/Game/Blueprint/Interactable/Building/EBuildingVisualGroupMode` (`self.Mode`)
    (:`NewEnumerator3`
      (`self.SetVisibility` `Is Construction Completed` true))
    (:`NewEnumerator0`
      (`self.SetVisibility` (< `Construction Percent` _construction_threshold) true))
    (:`NewEnumerator1`
      (`self.SetVisibility` (>= `Construction Percent` _construction_threshold) true))))