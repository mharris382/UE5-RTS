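; Windmill building Blueprint that shows and spins its sail once construction is complete.
; Each Tick it checks the build percent, hiding the sail mesh while the building is unfinished.
; At full build it makes the sail visible and rotates it around local pitch by a spin rate scaled with delta time.
; The construction script only calls the parent.
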(event `self.ReceiveTick`
  (params (DeltaSeconds :type "Float (single-precision)"))
  (`parent.ReceiveTick` DeltaSeconds)
  (if (>= (`self.Get Build Percent`) 1.0)
    (`SceneComponent.SetVisibility` (`self.SM_BLD_windmill_sail`) true false)
    (`SceneComponent.K2_AddLocalRotation` (`self.SM_BLD_windmill_sail`) (`KismetMathLibrary.MakeRotator` 0.0 (* DeltaSeconds (`self.Spin Rate`))) false false)
    (else
      (`SceneComponent.SetVisibility` (`self.SM_BLD_windmill_sail`) false false))))

(fn `UserConstructionScript`
  (`parent.UserConstructionScript`))