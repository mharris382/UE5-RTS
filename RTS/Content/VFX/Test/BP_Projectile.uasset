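; Test projectile actor that carries a Niagara firebolt effect and winds it down after its first bounce.
; Tick keeps the effect's Z axis pointing at world up, whatever the projectile's rotation.
; The first bounce plays a timeline that lerps Dissipation down before destroying the actor, while a parallel delay switches Emitting off.
; Velocity-based orientation, repositioning and size interpolation logic is left disconnected.
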(event `self.ReceiveBeginPlay`
  (set `self.last t` -1.0)
  (add `ProjectileMovementComponent.OnProjectileBounce` (`self.ProjectileMovement`) (delegate `On bounce`)))

(event `On bounce`
  (params (ImpactResult :type "HitResult Structure (by ref)") (ImpactVelocity :type "Vector Structure (by ref)"))
  (`/Engine/EditorBlueprintResources/StandardMacros.DoOnce` false
    (:`Completed`
      (`|ExecutionSequence`
        (:`then_0`
          (bind (_direction _effect) (`Timeline|Stop Effect`)
            (:`Update`
              (`NiagaraComponent.SetVariableFloat` (`self.NS_TestFireBolt`) "Dissipation" (`KismetMathLibrary.Lerp` 1.0 0.0 _effect)))
            (:`Finished`
              (`KismetSystemLibrary.Delay` 1.0)
              (`self.K2_DestroyActor`))))
        (:`then_1`
          (`KismetSystemLibrary.Delay` 2.5)
          (`NiagaraComponent.SetVariableBool` (`self.NS_TestFireBolt`) "Emitting" false))))))

(event `self.ReceiveHit`
  (params (MyComp :type "PrimitiveComponent Object Reference") (Other :type "Actor Object Reference") (OtherComp :type "PrimitiveComponent Object Reference") (bSelfMoved :type Boolean) (HitLocation :type "Vector Structure") (HitNormal :type "Vector Structure") (NormalImpulse :type "Vector Structure") (Hit :type "HitResult Structure (by ref)")))

(event `self.ReceiveTick`
  (params (DeltaSeconds :type "Float (single-precision)"))
  (`SceneComponent.K2_SetWorldRotation` (`self.NS_TestFireBolt`) (`KismetMathLibrary.MakeRotFromZ` (`KismetMathLibrary.Vector_Up`)) false false))

(fn `UserConstructionScript`)